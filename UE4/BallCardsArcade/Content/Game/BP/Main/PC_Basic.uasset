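; PC_Basic is a player controller that passes ball move and jump commands to the controlled BP_Player.
; MoveBall and JumpBall cast the controlled pawn to BP_Player, then call Move with a direction or TryJump.
; Both act only while the Input flag is true; the enable and disable override functions set that flag alongside engine input.
; It binds no input events itself, and its Tick is empty.
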(fn `DisableInputOverride`
  (`self.DisableInput` self)
  (set `self.bInput` false))

(fn `EnableInputOverride`
  (`self.EnableInput` self)
  (set `self.bInput` true))

(fn `JumpBall`
  (if (`self.bInput`)
    (bind _asbp_player (cast `/Game/Game/BP/WorldActor/BP_Player` (`self.K2_GetPawn`)))
    (`/Game/Game/BP/WorldActor/BP_Player.TryJump` _asbp_player)))

(fn `MoveBall`
  (params (dir :type "Float (double-precision)"))
  (if (`self.bInput`)
    (bind _asbp_player (cast `/Game/Game/BP/WorldActor/BP_Player` (`self.K2_GetPawn`)))
    (`/Game/Game/BP/WorldActor/BP_Player.Move` _asbp_player dir true)))

(fn `UserConstructionScript`)