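; BP_MenuCamera is a menu camera actor that moves between a default view and rooms along shop and beauty spline paths.
; GoTo selects a target room, and the FloatToRoom timeline drives the camera's transform along that room's spline.
; Switching between rooms reverses the current path to the default before playing the new one forward, then calls the room-reached event on arrival.
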(event `GoToGoal`
  (set `self.CurrentRoom` (`self.GoalRoom`))
  (set `self.CurrentSpline` (`|GetArrayItem` (`self.CamPaths`) (`KismetMathLibrary.Conv_ByteToInt` (`self.GoalRoom`))))
  (bind (_direction _duration) (`Timeline|FloatToRoom` :!label _label)
    (:`Update`
      (`SceneComponent.K2_SetWorldTransform` (`self.Camera`) (`SplineComponent.GetTransformAtTime` (`self.CurrentSpline`) _duration "World" false false) false false))
    (:`Finished`
      (if (== (`self.CurrentRoom`) (`self.GoalRoom`))
        (`self.RoomReachedEvent`)
        (else
          (`self.GoToGoal`))))))

(event `GoToDefault`
  (set `self.CurrentRoom` "NewEnumerator0")
  (goto _label :!via `Reverse`))

(event `GoTo`
  (params (Room :type "/Game/Game/BP/Enum/Menu/E_RoomsInMenu Enum" :default "NewEnumerator0"))
  (set `self.GoalRoom` Room)
  (if (!= (`self.GoalRoom`) (`self.CurrentRoom`))
    (if (!= 0 (`self.CurrentRoom`))
      (`self.GoToDefault`)
      (else
        (`self.GoToGoal`)))
    (else
      (`self.RoomReachedEvent`))))

(fn `UserConstructionScript`
  (set `self.CamPaths` (`|MakeArray` null (`self.ShopPath`) (`self.BeautyPath`))))