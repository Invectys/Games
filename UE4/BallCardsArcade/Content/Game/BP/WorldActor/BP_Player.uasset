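; Player pawn, a physics-driven ball that rolls along X and jumps, with a skin material from a data table.
; Each tick a downward sphere trace sets ground state and normal, gating movement impulses and orienting grounded jumps.
; An AbilityVars struct drives impulse strengths, air jumps and air float, with setters and a saved copy for reset.
; It also handles game-state input locking, debug cheats and tap-to-jump, while split-screen touch controls are left disconnected.
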(event `self.ReceiveBeginPlay`
  (bind _springarm (`self.SpringArm`))
  ;[1 1 1] BasicEvents
  (`|ExecutionSequence`
    (:`then_0`
      (set `PlayerController.bShowMouseCursor` (`self.ShowMouseCursor`) (`GameplayStatics.GetPlayerController` 0))
      (set `self.StartSpringArmLength` (`SpringArmComponent.TargetArmLength` _springarm))
      (set `self.StartTargetOffset` (`SpringArmComponent.TargetOffset` _springarm)))
    (:`then_1`
      (`self.IgnoreCollisionCheat`)
      (`self.HandleSelectedSkin`)
      ;;[1 1 1] SaveStartVars
      (set `self.AbilityVarsStart` (`self.AbilityVars`)))
    (:`then_2`
      ;;[1 1 1] TouchInput
      (if (`self.ActivateTouchInput`)
        (`PlayerController.ActivateTouchInterface` (`GameplayStatics.GetPlayerController` 0) (`self.TouchInput`))))))

(event `Key|Three`
  (params (Key :type "Key Structure"))
  ;[1 1 1] DebugKeys
  (:`Pressed`
    (if (`self.DebugKeys`)
      (bind _isa (`/Engine/EditorBlueprintResources/StandardMacros.FlipFlop`)
        (:`A`
          _)
        (:`B`
          _))
      (set `PlayerController.bShowMouseCursor` _isa (`GameplayStatics.GetPlayerController` 0)))))

(event `Key|Two`
  (params (Key :type "Key Structure"))
  ;[1 1 1] DebugKeys
  (:`Pressed`
    (if (`self.DebugKeys`)
      (`/Game/Game/BP/Main/GS_Play.LunchState` (`/Game/Game/BP/Function/FL_Standart.GSPlay`) "NewEnumerator2"))))

(event `Key|One`
  (params (Key :type "Key Structure"))
  ;[1 1 1] DebugKeys
  (:`Pressed`
    (if (`self.DebugKeys`)
      (bind _isa (`/Engine/EditorBlueprintResources/StandardMacros.FlipFlop`)
        (:`A`
          _)
        (:`B`
          _))
      (set `self.FlyCheat` _isa))))

(event `Key|Four`
  (params (Key :type "Key Structure"))
  (bind _asgi_instance (`/Game/Game/BP/Function/FL_Standart.GI`))
  ;[1 1 1] DebugKeys
  (:`Pressed`
    (if (`self.DebugKeys`)
      (`/Game/Game/BP/Main/GI_Instance.SetHaveCards` _asgi_instance (`/Game/Game/BP/Main/GI_Instance.CardsPacket1` _asgi_instance)))))

(event `self.ReceiveTick`
  (params (DeltaSeconds :type "Float (single-precision)"))
  ;[1 1 1] BasicEvents
  (`|ExecutionSequence`
    (:`then_0`
      (`self.CheckGround`)
      (if (`self.onGround`)
        (set `self.CurrentJumpInAirCount` 0)))
    (:`then_1`
      ;;[1 1 1] TouchMove
      (`self.Move` (`self.MoveTouchDir`)))))

(event `/Game/Game/BP/Component/StateSys/IHasGameState.onStartGame`
  (bind _aspc_basic (`/Game/Game/BP/Function/FL_Standart.PCB`))
  ;[1 1 1] game events
  (`/Engine/EditorBlueprintResources/StandardMacros.IsValid` _aspc_basic
    (:`Is Valid`
      (`/Game/Game/BP/Main/PC_Basic.DisableInputOverride` _aspc_basic))))

(event `/Game/Game/BP/Component/StateSys/IHasGameState.onStartPlaying`
  ;[1 1 1] game events
  (`/Game/Game/BP/Main/PC_Basic.EnableInputOverride` (`/Game/Game/BP/Function/FL_Standart.PCB`)))

(event `InputAxis|Move`
  (params (AxisValue :type "Float (single-precision)"))
  ;[1 1 1] MovementKeyboard
  (`self.Move` AxisValue))

(event `InputAction|Jump`
  (params (Key :type "Key Structure"))
  ;[1 1 1] MovementKeyboard
  (:`Pressed`
    (`self.TryJump`)))

(event `/Game/Game/BP/Component/StateSys/IHasGameState.onEndGame`
  ;[1 1 1] game events
  (`/Game/Game/BP/Main/PC_Basic.DisableInputOverride` (`/Game/Game/BP/Function/FL_Standart.PCB`)))

(event `InputTouch`
  (params (Location :type "Vector Structure") (FingerIndex :type "ETouchIndex Enum"))
  (:`Pressed`
    (`self.TryJump`)))

(event `InputAction|SelectAbility`
  (params (Key :type "Key Structure"))
  (bind _ashud_game (`/Game/Game/BP/Function/FL_Standart.HGame`))
  ;[1 1 1] ShowSelectAbility
  (:`Pressed`
    (`/Engine/EditorBlueprintResources/StandardMacros.FlipFlop`
      (:`A`
        (`/Game/Game/BP/Main/HUD/HUD_Game.ShowSelectAbility` _ashud_game))
      (:`B`
        (`/Game/Game/BP/Main/HUD/HUD_Game.HideSelectAbility` _ashud_game)))))

(event `self.Mesh.OnComponentHit`
  (params (HitComponent :type "PrimitiveComponent Object Reference") (OtherActor :type "Actor Object Reference") (OtherComp :type "PrimitiveComponent Object Reference") (NormalImpulse :type "Vector Structure") (Hit :type "HitResult Structure (by ref)"))
  (bind _returnvalue (`KismetMathLibrary.VSize` NormalImpulse))
  (`KismetSystemLibrary.PrintString` (`KismetStringLibrary.Conv_DoubleToString` _returnvalue))
  (if (> _returnvalue 200.0)
    (`GameplayStatics.PlaySound2D` (`self.FallSound`) 1.0 1.0 0.0 null null)))

(fn `AddJumpImpulse`
  (params (add :type "Float (double-precision)"))
  (bind (_floatinair _jumpsinairmaxcount _floatinairimpulse _moveimpulse _jumpimpulse) (break `/Game/Game/Data/S_BallAbilityVars` (`self.AbilityVars`)))
  (`|VariableSetRef` _jumpimpulse (+ add _jumpimpulse)))

(fn `AddMoveImpulse`
  (params (add :type "Float (double-precision)"))
  (bind (_floatinair _jumpsinairmaxcount _floatinairimpulse _moveimpulse) (break `/Game/Game/Data/S_BallAbilityVars` (`self.AbilityVars`)))
  (`|VariableSetRef` _moveimpulse (+ _moveimpulse add)))

(fn `CheckGround`
  (bind _returnvalue (`self.K2_GetActorLocation`))
  (bind _relativescale3d_x (`KismetMathLibrary.BreakVector` (`SceneComponent.RelativeScale3D` (`self.Mesh`))))
  (bind (_outhit _returnvalue_2) (`KismetSystemLibrary.SphereTraceSingle` :`Start` _returnvalue :`End` (+ _returnvalue (`KismetMathLibrary.MakeVector` 0.0 0.0 (* (`self.GroundCheckLength`) -1.0))) :`Radius` (* (`self.RadiusGroundCheck`) _relativescale3d_x) :`TraceChannel` "TraceTypeQuery1" :`DrawDebugType` (`self.DrawCheckGroundTrace`)))
  (set `self.onGround` _returnvalue_2)
  (set `self.GroundNormal` (`.Normal` (`GameplayStatics.BreakHitResult` _outhit))))

(fn `getFloatInAir`
  (returns (FloatInAir :type Boolean))
  (return (`.FloatInAir_1_2580277245E84FB9469C2A93F5E2E467` (break `/Game/Game/Data/S_BallAbilityVars` (`self.AbilityVars`)))))

(fn `getFloatInAirImpulse`
  (returns (impulse :type "Float (double-precision)"))
  (return (`.FloatInAirImpulse_7_DCD205B849D37F71DD3B2CAF628577CE` (break `/Game/Game/Data/S_BallAbilityVars` (`self.AbilityVars`)))))

(fn `getJumpImpulse`
  (returns (JumpImpulse :type "Float (double-precision)"))
  (return (`.JumpImpulse_11_907A9AC54B95C16BAABF61B01D4EF489` (break `/Game/Game/Data/S_BallAbilityVars` (`self.AbilityVars`)))))

(fn `getJumpsInAirMaxCount`
  (returns (MaxJumps :type Integer))
  (return (`.JumpsInAirMaxCount_4_4486B7FA42916743F5A53F843C0FFCDF` (break `/Game/Game/Data/S_BallAbilityVars` (`self.AbilityVars`)))))

(fn `getMoveImpulse`
  (returns (impulse :type "Float (double-precision)"))
  (return (`.MoveImpulse_9_A8D40CDD4AA90A8AF61E5C858246094A` (break `/Game/Game/Data/S_BallAbilityVars` (`self.AbilityVars`)))))

(fn `GetStartVars`
  (returns (AbilityVarsStart :type "/Game/Game/Data/S_BallAbilityVars Structure"))
  (return (`self.AbilityVarsStart`)))

(fn `HandleSelectedSkin`
  (if (`self.SetSelectedSkin`)
    (`self.SetSkin` (`/Game/Game/BP/Main/GI_Instance.getSelectedSkin` (`/Game/Game/BP/Function/FL_Standart.GI`)))))

(fn `IgnoreCollisionCheat`
  (if (`self.IgnoreObstacles`)
    (`PrimitiveComponent.SetCollisionResponseToChannel` (`self.Mesh`) "ECC_WorldStatic" "ECR_Ignore")
    (else
      (`PrimitiveComponent.SetCollisionResponseToChannel` (`self.Mesh`) "ECC_WorldStatic" "ECR_Block"))))

(fn `Jump`
  (params (dirrection :type "Vector Structure"))
  (`self.JumpImpulseMethod` dirrection)
  (`GameplayStatics.PlaySound2D` (`self.JumpSound`) 1.0 1.0 0.0 null null))

(fn `JumpImpulseMethod`
  (params (dirrection :type "Vector Structure"))
  (`PrimitiveComponent.AddImpulse` (`self.Mesh`) (* dirrection (`self.getJumpImpulse`)) "None" false))

(fn `Move`
  (params (dir :type "Float (double-precision)") (Condition :type Boolean :default true))
  (locals (dir_ :type "Float (double-precision)"))
  (set `local.dir_` dir)
  (`self.MoveImpulseMethod` (`local.dir_`) (and Condition (or (`self.getFloatInAir`) (`self.onGround`) (`self.FlyCheat`))) (* (`GameplayStatics.GetWorldDeltaSeconds`) (`KismetMathLibrary.SelectFloat` (`self.getFloatInAirImpulse`) (`self.getMoveImpulse`) (and (`self.getFloatInAir`) (not (`self.onGround`)))) 50.0)))

(fn `MoveImpulseMethod`
  (params (dir :type "Float (double-precision)") (Condition :type Boolean) (Impulse :type "Float (double-precision)"))
  (if (and Condition (!= dir 0.0))
    (`PrimitiveComponent.AddImpulse` (`self.Mesh`) (* (* (`KismetMathLibrary.MakeVector` 1.0) Impulse) dir) "None" false)))

(fn `ResetAbilityVars`
  (set `self.AbilityVars` (`self.AbilityVarsStart`)))

(fn `SetFloatInAir`
  (params (Enable :type Boolean) (Set :type "Float (double-precision)"))
  (bind (_floatinair _jumpsinairmaxcount _floatinairimpulse) (break `/Game/Game/Data/S_BallAbilityVars` (`self.AbilityVars`)))
  (`|VariableSetRef` _floatinair Enable)
  (`|VariableSetRef` _floatinairimpulse Set))

(fn `SetJumpImpulse`
  (params (newImpulse :type "Float (double-precision)"))
  (setmembers `/Game/Game/Data/S_BallAbilityVars` :`StructRef` (`self.AbilityVars`) :`JumpImpulse` newImpulse))

(fn `SetJumpsMaxCount`
  (params (JumpsInAirCount :type Integer))
  (`|VariableSetRef` (`.JumpsInAirMaxCount_4_4486B7FA42916743F5A53F843C0FFCDF` (break `/Game/Game/Data/S_BallAbilityVars` (`self.AbilityVars`))) JumpsInAirCount))

(fn `SetMoveImpulse`
  (params (MoveImpulse :type "Float (double-precision)"))
  (setmembers `/Game/Game/Data/S_BallAbilityVars` :`StructRef` (`self.AbilityVars`) :`MoveImpulse` MoveImpulse))

(fn `SetSkin`
  (params (Row :type Name))
  (bind _returnvalue (`|GetDataTableRow` "/Game/Game/Data/DT_SkinsData.DT_SkinsData" Row)
    (:`then`
      (`PrimitiveComponent.SetMaterial` (`self.Mesh`) 0 (`.Material_5_AAF8FDD64D93F34A91EBC1A3779F8924` (break `/Game/Game/Data/S_SkinInfo` _returnvalue))))))

(fn `TryJump`
  (locals (dir :type "Vector Structure" :default (0.0 0.0 0.0)))
  (`|ExecutionSequence`
    (:`then_0`
      (if (not (`self.onGround`))
        (set `local.dir` (0.0 0.0 1.0))
        (else
          (set `local.dir` (`self.GroundNormal`)))))
    (:`then_1`
      (if (or (`self.onGround`) (< (`self.CurrentJumpInAirCount`) (`self.getJumpsInAirMaxCount`)) (`self.FlyCheat`))
        (`self.Jump` (`local.dir`))
        (`/Engine/EditorBlueprintResources/StandardMacros.IncrementInt` (`self.CurrentJumpInAirCount`))))))

(fn `UserConstructionScript`)