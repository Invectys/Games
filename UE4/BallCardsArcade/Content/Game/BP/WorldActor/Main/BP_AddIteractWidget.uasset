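; BP_AddIteractWidget is a world Blueprint that shows and hides a W_GameTrader widget through its Toggle event.
; Toggling on lazily creates the widget with the Blueprint's item Type and Row, caches it, and adds it to the viewport.
; Toggling off removes it from its parent but keeps the reference, so later toggles reuse the same instance while it remains valid.
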(event `/Game/Game/BP/Component/interface/IToggled.Toggle`
  (params (on :type Boolean))
  (`KismetSystemLibrary.PrintString` (`KismetStringLibrary.Conv_BoolToString` on) false false)
  (if on
    (`|ExecutionSequence`
      (:`then_0`
        (`/Engine/EditorBlueprintResources/StandardMacros.IsValid` (`self.Widget`)
          (:`Is Not Valid`
            (bind _returnvalue (`|CreateWidget` "/Game/Game/BP/Widget/W_GameTrader.W_GameTrader_C" null (`self.Type`) (`self.Row`)))
            (set `self.Widget` _returnvalue))))
      (:`then_1`
        (`UserWidget.AddToViewport` (`self.Widget`) 1)))
    (else
      (`Widget.RemoveFromParent` (`self.Widget`)))))

(fn `UserConstructionScript`)