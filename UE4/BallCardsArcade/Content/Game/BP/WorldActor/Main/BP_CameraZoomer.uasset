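; BP_CameraZoomer is a placeable trigger volume that changes the player camera's zoom and offset while the player is inside its box.
; Box overlap events cache the BP_Player and toggle a Zoom flag.
; Tick continuously interpolates the player's spring arm length and target offset toward either the zoom values or the player's stored start values, each at its own speed.
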(event `self.ReceiveTick`
  (params (DeltaSeconds :type "Float (single-precision)"))
  (bind _player (`self.Player`))
  (bind _player_2 (`self.Player`))
  (bind _springarm (`/Game/Game/BP/WorldActor/BP_Player.SpringArm` (`self.Player`)))
  (`/Engine/EditorBlueprintResources/StandardMacros.IsValid` (`self.Player`)
    (:`Is Valid`
      (set `SpringArmComponent.TargetArmLength` (`KismetMathLibrary.FInterpTo` (`SpringArmComponent.TargetArmLength` (`/Game/Game/BP/WorldActor/BP_Player.SpringArm` _player_2)) (`KismetMathLibrary.SelectFloat` (`self.ZoomLength`) (`/Game/Game/BP/WorldActor/BP_Player.StartSpringArmLength` _player_2) (`self.Zoom`)) (`GameplayStatics.GetWorldDeltaSeconds`) (`self.Speed`)) _springarm)
      (set `SpringArmComponent.TargetOffset` (`KismetMathLibrary.VInterpTo` (`SpringArmComponent.TargetOffset` (`/Game/Game/BP/WorldActor/BP_Player.SpringArm` _player)) (`KismetMathLibrary.SelectVector` (`self.ZoomOffset`) (`/Game/Game/BP/WorldActor/BP_Player.StartTargetOffset` _player) (`self.Zoom`)) (`GameplayStatics.GetWorldDeltaSeconds`) (`self.SpeedOffset`)) _springarm))))

(event `self.Box.OnComponentBeginOverlap`
  (params (OverlappedComponent :type "PrimitiveComponent Object Reference") (OtherActor :type "Actor Object Reference") (OtherComp :type "PrimitiveComponent Object Reference") (OtherBodyIndex :type Integer) (bFromSweep :type Boolean) (SweepResult :type "HitResult Structure (by ref)"))
  (bind _asbp_player (cast `/Game/Game/BP/WorldActor/BP_Player` OtherActor))
  (set `self.Player` _asbp_player)
  (set `self.Zoom` true))

(event `self.Box.OnComponentEndOverlap`
  (params (OverlappedComponent :type "PrimitiveComponent Object Reference") (OtherActor :type "Actor Object Reference") (OtherComp :type "PrimitiveComponent Object Reference") (OtherBodyIndex :type Integer))
  (bind _asbp_player (cast `/Game/Game/BP/WorldActor/BP_Player` OtherActor))
  (set `self.Player` _asbp_player)
  (set `self.Zoom` false))

(fn `UserConstructionScript`)