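; BP_Password2 is a two-button password mechanism that generates a random on/off combination at BeginPlay.
; It binds to the toggle events of two linked switcher buttons and stores each state in a Current array.
; Every toggle compares Current against Password and passes the match result to EnableSwitcher, so the mechanism is enabled only while the combination is correct.
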(event `self.ReceiveBeginPlay`
  (`parent.ReceiveBeginPlay`)
  (add `self.Toggle` (`/Game/Game/BP/Function/FL_Standart.castGSwither` (`self.BP_Button1`)) (delegate `Toggle1`))
  (add `self.Toggle` (`/Game/Game/BP/Function/FL_Standart.castGSwither` (`self.BP_Button2`)) (delegate `Toggle2`))
  (`self.GeneratePassword`))

(event `Toggle1` :!signature `self.Toggle`
  (params (Enabled :type Boolean))
  (`KismetArrayLibrary.Array_Set` (`self.Current`) 0 Enabled true)
  (`self.Check`))

(event `Toggle2` :!signature `self.Toggle`
  (params (Enabled :type Boolean))
  (`KismetArrayLibrary.Array_Set` (`self.Current`) 1 Enabled true)
  (`self.Check`))

(event `Check`
  (`self.EnableSwitcher` (`KismetArrayLibrary.Array_Identical` (`self.Password`) (`self.Current`))))

(fn `GeneratePassword`
  (set `self.Password` (`|MakeArray` (`KismetMathLibrary.RandomBool`) (`KismetMathLibrary.RandomBool`))))

(fn `UserConstructionScript`
  (`parent.UserConstructionScript`))