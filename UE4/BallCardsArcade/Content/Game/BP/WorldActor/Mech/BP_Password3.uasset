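; BP_Password3 is a world mech puzzle Blueprint that extends a parent password actor with a third switch-driven boolean slot.
; On BeginPlay it binds to the toggle event of BPButton3, whose state is written into Current at index 2 before calling Check.
; GeneratePassword runs the parent version, then randomizes the same Password index, so each child layer adds one element to the code.
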(event `self.ReceiveBeginPlay`
  (`parent.ReceiveBeginPlay`)
  (add `/Game/Game/BP/WorldActor/Mech/BP_Switchers.Toggle` (`/Game/Game/BP/Function/FL_Standart.castGSwither` (`self.BP_Button3`)) (delegate `CustomEvent`)))

(event `CustomEvent`
  (params (Enabled :type Boolean))
  (`KismetArrayLibrary.Array_Set` (`self.Current`) 2 Enabled true)
  (`self.Check`))

(fn `GeneratePassword`
  (`parent.GeneratePassword`)
  (`KismetArrayLibrary.Array_Set` (`self.Password`) 2 (`KismetMathLibrary.RandomBool`) true)
  (for _array_element (`self.Password`)
    (`KismetSystemLibrary.PrintString` (`KismetStringLibrary.Conv_BoolToString` _array_element) false false (struct :`G` 0.66 :`B` 1.0 :`A` 1.0) 11.0)))

(fn `UserConstructionScript`
  (`parent.UserConstructionScript`))