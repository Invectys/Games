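; BP_Trampoline is a world actor that acts as a trampoline, applying a bounce impulse to components that hit it.
; On a hit of the Sphere component, it scales the hit's normal impulse per axis by the absolute Arrow forward vector, then by TrampolineIm.
; The result goes to the other component as a mass-dependent physics impulse.
; The construction script sets Sphere's static mesh from the Mesh variable.
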(event `self.Sphere.OnComponentHit`
  (params (HitComponent :type "PrimitiveComponent Object Reference") (OtherActor :type "Actor Object Reference") (OtherComp :type "PrimitiveComponent Object Reference") (NormalImpulse :type "Vector Structure") (Hit :type "HitResult Structure (by ref)"))
  (`PrimitiveComponent.AddImpulse` OtherComp (* (* NormalImpulse (`KismetMathLibrary.Vector_GetAbs` (`SceneComponent.GetForwardVector` (`self.Arrow`)))) (`self.trampolineIm`)) "None" false))

(fn `UserConstructionScript`
  (`StaticMeshComponent.SetStaticMesh` (`self.Sphere`) (`self.Mesh`)))