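; BP_ElemMech1 is a Level 1 procedural element actor that links a switch to three gates.
; On BeginPlay it binds its Toggle event to the switcher obtained by casting BPButton.
; Toggle forwards the enabled state through ToggleMessage to the child actors of BPGate1, BPGate2 and BPGate in that order, with short delays between calls to stagger the gates.
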(event `self.ReceiveBeginPlay`
  (`parent.ReceiveBeginPlay`)
  (add `/Game/Game/BP/WorldActor/Mech/BP_Switchers.Toggle` (`/Game/Game/BP/Function/FL_Standart.castGSwither` (`self.BP_Button`)) (delegate `Toggle`)))

(event `Toggle`
  (params (Enabled :type Boolean))
  (message `/Game/Game/BP/Component/interface/IToggled.Toggle` (`ChildActorComponent.ChildActor` (`self.BP_Gate1`)) Enabled)
  (`KismetSystemLibrary.Delay` 0.2)
  (message `/Game/Game/BP/Component/interface/IToggled.Toggle` (`ChildActorComponent.ChildActor` (`self.BP_Gate2`)) Enabled)
  (`KismetSystemLibrary.Delay` 0.2)
  (message `/Game/Game/BP/Component/interface/IToggled.Toggle` (`ChildActorComponent.ChildActor` (`self.BP_Gate`)) Enabled))

(fn `UserConstructionScript`
  (`parent.UserConstructionScript`))