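; BP_Elem_Door_2 is a Level 2 procedural element that pairs a button-operated gate with a spawner of blue cubes.
; On BeginPlay it registers the gate's child actor as the toggle target of BPButton's switcher.
; It also starts the CSpawnerLoop component spawning BP_BlueCube at the Point component's transform, using a short duration and a fixed count.
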(event `self.ReceiveBeginPlay`
  (`/Game/Game/BP/Function/FL_Standart.setToggleActorForSwitcher` (`self.BP_Button`) (`|MakeArray` (`ChildActorComponent.ChildActor` (`self.BP_Gate`))))
  (`/Game/Game/BP/Component/C_SpawnerLoop.SpawnLoop` (`self.C_SpawnerLoop`) 3 (`SceneComponent.K2_GetComponentToWorld` (`self.Point`)) "/Game/Game/BP/WorldActor/Secondary/BP_BlueCube.BP_BlueCube_C" 0.2))

(fn `UserConstructionScript`
  (`parent.UserConstructionScript`))