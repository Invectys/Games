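; BP_Card_ is a world pickup actor that grants the player one card.
; On BeginPlay it optionally picks a random row from the GameInstance's card rows, then applies that row's material to its mesh.
; When picked up, it adds the card through the GameInstance and spawns a HUD "+1 Card" popup at its location, plus an optional extra text popup just below.
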(event `self.ReceiveBeginPlay`
  (bind _cardsrows (`/Game/Game/BP/Main/GI_Instance.getCardsRows` (`/Game/Game/BP/Function/FL_Standart.GI`)))
  (bind (_out_row_cardname _out_row_description _out_row_image _out_row_material) (break `/Game/Game/Data/S_CardInfo` (`/Game/Game/BP/Function/FL_Data.getCardRow` (`self.CardRow`))))
  (`parent.ReceiveBeginPlay`)
  (`|ExecutionSequence`
    (:`then_0`
      (if (`self.RandomCard`)
        (bind _output_get (set `self.CardRow` (`|GetArrayItem` _cardsrows (`KismetMathLibrary.RandomInteger` (`KismetArrayLibrary.Array_Length` _cardsrows)))))
        (`KismetSystemLibrary.PrintString` (`KismetStringLibrary.Conv_NameToString` _output_get) false false)))
    (:`then_1`
      (`PrimitiveComponent.SetMaterial` (`self.StaticMesh1`) 0 _out_row_material))))

(event `self.Picked up`
  (params (Player :type "/Game/Game/BP/WorldActor/BP_Player Object Reference"))
  (`/Game/Game/BP/Main/GI_Instance.AddCard` (`/Game/Game/BP/Function/FL_Standart.GI`) (`self.CardRow`) 1)
  (`/Game/Game/BP/Main/HUD/HUD_Basic.SpawnPickupWidget` (`/Game/Game/BP/Function/FL_Standart.HBasic`) (`self.K2_GetActorLocation`) "<bonus>+1 Card </>")
  (if (`self.Additive`)
    (`/Game/Game/BP/Main/HUD/HUD_Basic.SpawnPickupWidget` (`/Game/Game/BP/Function/FL_Standart.HBasic`) (- (`self.K2_GetActorLocation`) (0.0 0.0 50.0)) (`self.TextAdditive`))))

(fn `UserConstructionScript`
  (`parent.UserConstructionScript`))