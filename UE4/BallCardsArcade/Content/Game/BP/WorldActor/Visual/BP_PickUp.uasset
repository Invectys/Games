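; BP_PickUp is a short-lived visual actor that displays floating pickup text and removes itself after a few seconds.
; On BeginPlay it stores its start location and passes its Text to a W_Pickup widget.
; Each Tick drifts it from that origin along X and Z using linear-plus-sine math expressions, with X offset and scaled.
; Speed is added per frame, so the motion depends on frame rate.
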(event EventBeginPlay
  (Variables|Movement|SetStartLoc (Transformation|GetActorLocation))
  (Actor|SetLifeSpan 5.0)
  ;[1 1 1] WidgetInfo
  (bind _asw_pickup (Utilities|Casting|CastToW_Pickup (UserInterface|GetUserWidgetObject (Variables|Default|GetWidget))))
  (Default|SetText _asw_pickup (Variables|Default|GetText)))

(event EventTick
  (params (DeltaSeconds :type Float%20%28single-precision%29))
  (Variables|Movement|SetTime (+ DeltaSeconds (Variables|Movement|GetTime) (Variables|Movement|GetSpeed)))
  ;[1 1 1] Movement
  (Transformation|SetActorLocation (+ (Math|Vector|MakeVector (* (|(x+(30*(sin((x/10))))) (- (Variables|Movement|GetTime) (Variables|Movement|GetYDelta))) (Variables|Movement|GetYAcseleration)) 0.0 (|(x+(30*(sin((x/10))))) (Variables|Movement|GetTime))) (Variables|Movement|GetStartLoc)) false false))

(fn ConstructionScript)