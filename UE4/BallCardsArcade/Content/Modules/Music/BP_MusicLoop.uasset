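; BP_MusicLoop plays a music cue as non-spatial 2D sound and repeats it with a pause between plays.
; On BeginPlay it calls Lunch if music is enabled in GI and AutoLunch is set.
; Lunch creates and plays a new audio component, whose finish event waits PlayDelay and calls Lunch again without rechecking the music setting.
; Destroy removes the current audio component.
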(event `self.ReceiveBeginPlay`
  (if (`/Game/Game/BP/Main/GI_Instance.MusicEnabled` (`/Game/Game/BP/Function/FL_Standart.GI`))
    (if (`self.AutoLunch`)
      (`self.Lunch`))))

(event `AudioFinish`
  (`KismetSystemLibrary.Delay` (`self.PlayDelay`))
  (`self.Lunch`))

(fn `Destroy`
  (`ActorComponent.K2_DestroyComponent` (`self.AudioComponent`)))

(fn `Lunch`
  (bind _returnvalue (`GameplayStatics.CreateSound2D` (`self.Cue`) 1.0 1.0 0.0 null))
  (bind _output_get (set `self.AudioComponent` _returnvalue))
  (`AudioComponent.Play` _output_get 0.0)
  (add `AudioComponent.OnAudioFinished` (`self.AudioComponent`) (`|CreateDelegate` :!event `AudioFinish`)))

(fn `UserConstructionScript`)