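; BP_ActorsFloater is a world actor that moves a set of actors along a fixed direction each tick while enabled and working.
; An optional mode recomputes speed from the base speed plus Target-to-From distance, divided by a distance step scaled by delta time.
; Each FloatActors entry gets the same frame-time-scaled offset, without sweep.
; Toggle sets the enabled state, game end disables it, and the start events are empty.
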(event `self.ReceiveTick`
  (params (DeltaSeconds :type "Float (single-precision)"))
  (if (and (`self.Enabled`) (`self.Work`))
    (`|ExecutionSequence`
      (:`then_0`
        ;[1 1 1] CalckSpeed
        (if (`self.IncreaseSpeedifFar`)
          (set `self.Speed` (+ (`self.StartSpeed`) (/ (`KismetMathLibrary.Vector_Distance` (`self.K2_GetActorLocation` (`self.Target`)) (`self.K2_GetActorLocation` (`self.From`))) (* (`self.IncreaseDeltaDistance`) (`GameplayStatics.GetWorldDeltaSeconds`)))))))
      (:`then_1`
        ;[1 1 1] Offset
        (set `self.Offset` (* (`self.Dir`) (* (`GameplayStatics.GetWorldDeltaSeconds`) (`self.GetSpeed`))))
        ;[1 1 1] Move
        (for _array_element (`self.FloatActors`)
          (`self.K2_SetActorLocation` _array_element (+ (`self.K2_GetActorLocation` _array_element) (`self.Offset`)) false false))))))

(event `/Game/Game/BP/Component/StateSys/IHasGameState.onStartGame`)

(event `/Game/Game/BP/Component/StateSys/IHasGameState.onStartPlaying`)

(event `/Game/Game/BP/Component/interface/IToggled.Toggle`
  (params (on :type Boolean))
  (set `self.Enabled` on))

(event `/Game/Game/BP/Component/StateSys/IHasGameState.onEndGame`
  (set `self.Enabled` false))

(fn `GetDeathHeigth`
  (returns (Heigth :type "Float (double-precision)"))
  (return 0.0))

(fn `GetSpeed`
  (returns (Speed :type "Float (double-precision)"))
  (return (`self.Speed`)))

(fn `UserConstructionScript`)