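; BP_Finish is the map goal actor that completes the level when the player reaches it.
; Its overlap handler runs the parent logic, then continues only if the other actor is a BP_Player.
; It spawns a confetti effect offset from the actor and plays a 2D sound.
; It then calls FinishMap on the play game state, passing an end reason with description and the levels to unlock.
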(fn `OnOverlap`
  (params (OtherActor :type "Actor Object Reference"))
  (`parent.OnOverlap` OtherActor)
  (cast `/Game/Game/BP/WorldActor/BP_Player` OtherActor)
  (`GameplayStatics.SpawnEmitterAtLocation` "/Game/Game/Visual/Particles/P_Confetti.P_Confetti" (+ (`SceneComponent.K2_GetComponentLocation` (`self.DefaultSceneRoot`)) (0.0 100.0 0.0)))
  (`GameplayStatics.PlaySound2D` (`self.ConfettiSound`) 1.0 1.0 0.0 null null)
  (`/Game/Game/BP/Main/GS_Play.FinishMap` (`/Game/Game/BP/Function/FL_Standart.GSPlay`) (make `/Game/Game/Data/S_EndGame` "NewEnumerator0" (`self.EndDescription`)) (`self.UnlockLevels`)))

(fn `UserConstructionScript`)