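; BP_LocationSwitcher is a world actor that moves a Chaser actor to follow a Target's location.
; Every Tick it divides the Target position by SwithDelta and multiplies it back, apparently intended as grid stepping, though no explicit rounding appears.
; FollowX, FollowY and FollowZ select per axis whether the Chaser takes that value or keeps its own coordinate.
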(event `self.ReceiveTick`
  (params (DeltaSeconds :type "Float (single-precision)"))
  (bind _chaser (`self.chaser`))
  (bind (_returnvalue_x _returnvalue_y _returnvalue_z) (`KismetMathLibrary.BreakVector` (`self.K2_GetActorLocation` _chaser)))
  (bind (_returnvalue_x_2 _returnvalue_y_2 _returnvalue_z_2) (`KismetMathLibrary.BreakVector` (* (/ (`self.K2_GetActorLocation` (`self.target`)) (`self.SwithDelta`)) (`self.SwithDelta`))))
  (`self.K2_SetActorLocation` _chaser (`KismetMathLibrary.MakeVector` (`KismetMathLibrary.SelectFloat` _returnvalue_x_2 _returnvalue_x (`self.FollowX`)) (`KismetMathLibrary.SelectFloat` _returnvalue_y_2 _returnvalue_y (`self.FollowY`)) (`KismetMathLibrary.SelectFloat` _returnvalue_z_2 _returnvalue_z (`self.FollowZ`))) false false))

(fn `UserConstructionScript`)