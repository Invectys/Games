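; BP_ActivateZone is a trigger zone mechanism that turns a switcher on while the player is inside it.
; Overlap events on its Box component feed OnOverlap and OnEndOverlap, which filter for BP_Player and call EnableSwitcher with true on entry and false on exit.
; Its construction script only runs the parent's.
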(event `self.Box.OnComponentBeginOverlap`
  (params (OverlappedComponent :type "PrimitiveComponent Object Reference") (OtherActor :type "Actor Object Reference") (OtherComp :type "PrimitiveComponent Object Reference") (OtherBodyIndex :type Integer) (bFromSweep :type Boolean) (SweepResult :type "HitResult Structure (by ref)"))
  (`self.OnOverlap` OtherActor))

(event `self.Box.OnComponentEndOverlap`
  (params (OverlappedComponent :type "PrimitiveComponent Object Reference") (OtherActor :type "Actor Object Reference") (OtherComp :type "PrimitiveComponent Object Reference") (OtherBodyIndex :type Integer))
  (`self.OnEndOverlap` OtherActor))

(fn `OnEndOverlap`
  (params (Actor :type "Actor Object Reference"))
  (cast `/Game/Game/BP/WorldActor/BP_Player` Actor)
  (`self.EnableSwitcher` false))

(fn `OnOverlap`
  (params (OtherActor :type "Actor Object Reference"))
  (cast `/Game/Game/BP/WorldActor/BP_Player` OtherActor)
  (`self.EnableSwitcher` true))

(fn `UserConstructionScript`
  (`parent.UserConstructionScript`))