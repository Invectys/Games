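; BP_Button is a mechanism button that drives inherited switcher logic from the position of its Button component.
; Each tick it measures the distance between the Button's relative location and the actor's world location, counting as pressed below PressBorder.
; The pressed state, compared with the Reverse flag, feeds EnableSwitcher.
; The EnableActionsForOverride override calls the parent, then turns the point light green when enabled and red when disabled.
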(event `self.ReceiveTick`
  (params (DeltaSeconds :type "Float (single-precision)"))
  (`self.EnableSwitcher` (== (`self.IsPressed`) (`self.Reverse`))))

(fn `EnableActionsForOverride`
  (params (State :type Boolean))
  (bind _pointlight (`self.PointLight`))
  (`parent.EnableActionsForOverride` State)
  (if State
    (`LightComponent.SetLightColor` _pointlight (struct :`G` 1.0 :`A` 1.0) true)
    (else
      (`LightComponent.SetLightColor` _pointlight (struct :`R` 1.0 :`A` 1.0) true))))

(fn `GetPressValue`
  (returns (PressValue :type "Float (double-precision)"))
  (return (`KismetMathLibrary.VSize` (- (`SceneComponent.RelativeLocation` (`self.Button`)) (`self.K2_GetActorLocation`)))))

(fn `IsPressed`
  (returns (Pressed :type Boolean))
  (return (< (`self.GetPressValue`) (`self.PressBorder`))))

(fn `UserConstructionScript`)