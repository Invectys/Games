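; BP_Lever is a physical lever switch that turns on or off based on which side it is swung to.
; Each tick it checks the sign of the physics constraint's Swing2 angle, compares it to RightEnabling and passes the result to EnableSwitcher.
; Its EnableActionsForOverride calls the parent version, then colors a point light green when enabled or red when disabled.
; A helper macro branches execution on Left or Right position.
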(event `self.ReceiveTick`
  (params (DeltaSeconds :type "Float (single-precision)"))
  (`self.EnableSwitcher` (== (`self.GetLeverPosition_`) (`self.rightEnabling`))))

(fn `EnableActionsForOverride`
  (params (State :type Boolean))
  (bind _pointlight (`self.PointLight`))
  (`parent.EnableActionsForOverride` State)
  (if State
    (`LightComponent.SetLightColor` _pointlight (struct :`G` 1.0 :`A` 1.0) true)
    (else
      (`LightComponent.SetLightColor` _pointlight (struct :`R` 1.0 :`A` 1.0) true))))

(fn `GetLeverPosition_`
  (returns (Right :type Boolean))
  (return (>= (`PhysicsConstraintComponent.GetCurrentSwing2` (`self.PhysicsConstraint`)) 0.0)))

(fn `UserConstructionScript`)