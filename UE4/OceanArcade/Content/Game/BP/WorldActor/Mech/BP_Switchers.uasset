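; BP_Switchers is a switch actor base that turns linked world objects on or off.
; EnableSwitcher reacts only to input changes while Work is set, either following the input or, when Sticky, flipping Enabled on each switch-on.
; Once makes it single-use by clearing Work.
; The state goes to AToggle targets via ToggleMessage, then to the empty EnableActionsForOverride hook and CallToggle.
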(fn `EnableActionsForOverride`
  (params (State :type Boolean)))

(fn `EnableSwitcher`
  (params (on :type Boolean))
  (bind _enabled (`self.Enabled`))
  (if (and (!= on (`self.EnabledSwitcher`)) (`self.Work`))
    (`|ExecutionSequence`
      (:`then_0`
        (if (`self.Once`)
          (set `self.Work` false)))
      (:`then_1`
        (bind _output_get (set `self.EnabledSwitcher` on))
        (`|ExecutionSequence`
          (:`then_0`
            (if (`self.Sticky`)
              (if (`self.EnabledSwitcher`)
                (set `self.Enabled` (not (`self.Enabled`)))
                (else
                  (return)))
              (else
                (set `self.Enabled` _output_get))))
          (:`then_1`
            (`|ExecutionSequence`
              (:`then_0`
                (for _array_element (`self.AToggle`)
                  (`/Engine/EditorBlueprintResources/StandardMacros.IsValid` _array_element
                    (:`Is Valid`
                      (message `/Game/Game/BP/Component/interface/IToggled.Toggle` _array_element _enabled)
                      (`KismetSystemLibrary.PrintString` (`KismetStringLibrary.Conv_BoolToString` _enabled) false false)))))
              (:`then_1`
                (`self.EnableActionsForOverride` (`self.Enabled`))
                (`self.Toggle` _enabled)))))))))

(fn `SetWork`
  (params (Work :type Boolean))
  (set `self.Work` Work))

(fn `UserConstructionScript`)