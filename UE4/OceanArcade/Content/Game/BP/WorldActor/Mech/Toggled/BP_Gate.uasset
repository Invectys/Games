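; BP_Gate is a toggleable gate actor that slides its Door component between a closed and an offset position.
; The construction script records the door's relative location as the start and adds Offset to get the end.
; The Toggle event plays or reverses the DoorAnim timeline, whose track lerps the door between those points by teleporting without sweep.
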(event `/Game/Game/BP/Component/interface/IToggled.Toggle`
  (params (on :type Boolean))
  (if on
    (bind (_direction _newtrack_0) (`Timeline|DoorAnim` :!label _label)
      (:`Update`
        (`SceneComponent.K2_SetRelativeLocation` (`self.door`) (`KismetMathLibrary.VLerp` (`self.StartPos`) (`self.EndPos`) _newtrack_0) false true)))
    (else
      (goto _label :!via `Reverse`))))

(fn `UserConstructionScript`
  (bind _output_get (set `self.StartPos` (`SceneComponent.RelativeLocation` (`self.door`))))
  (set `self.EndPos` (+ _output_get (`self.Offset`))))