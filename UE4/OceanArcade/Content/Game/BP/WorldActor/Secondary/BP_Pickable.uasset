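; BP_Pickable is a world pickup that the player collects by walking into its PickUpSphere.
; A BP_Player overlap fires PickedUp, which calls PickedUpEvent with the player and itself, then plays a sound and destroys the actor.
; When PickupOnce is set, it also records a key on pickup and checks that key on BeginPlay, tracking one-time collection.
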(event `self.ReceiveBeginPlay`
  (if (`self.PickupOnce`)
    (`/Game/Game/BP/Function/FL_LevelVariblesChecker.CheckKey` self "NewEnumerator1")))

(event `self.PickUpSphere.OnComponentBeginOverlap`
  (params (OverlappedComponent :type "PrimitiveComponent Object Reference") (OtherActor :type "Actor Object Reference") (OtherComp :type "PrimitiveComponent Object Reference") (OtherBodyIndex :type Integer) (bFromSweep :type Boolean) (SweepResult :type "HitResult Structure (by ref)"))
  (bind _asbp_player (cast `/Game/Game/BP/WorldActor/BP_Player` OtherActor))
  (`self.Picked up` _asbp_player)
  (`|ExecutionSequence`
    (:`then_0`
      (if (`self.PickupOnce`)
        (`/Game/Game/BP/Function/FL_LevelVariblesChecker.AddKey` self "NewEnumerator1")))
    (:`then_1`
      (`GameplayStatics.PlaySound2D` (`self.PickupSound`) 1.0 1.0 0.0 null null)
      (`self.K2_DestroyActor`))))

(event `Picked up`
  (params (Player :type "/Game/Game/BP/WorldActor/BP_Player Object Reference"))
  (`self.PickedUpEvent` Player self))

(fn `UserConstructionScript`)